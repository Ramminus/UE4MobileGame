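; Dialogue controller Blueprint that registers itself on the RPG game instance and starts and ends dialogue on the player's HUD.
; It disables its input on BeginPlay and enables it when a dialogue initializes, after calling the parent implementation.
; Construction sets a sentence replacement with a hard-coded player name.
; ReplaceText and the Space key handler only print strings, the former substituting the name placeholder in the first sentence.
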(event EventBeginPlay
  ;[1 1 1] Set Game Instance Reference
  (bind _asrpggame_instance (Utilities|Casting|CastToRPGGameInstance (Game|GetGameInstance)))
  (bind _output_get (Variables|/Game/Blueprints/RPGGameInstance.RPGGameInstance_C|SetDialogueController _asrpggame_instance self))
  (Input|DisableInput _output_get (Game|GetPlayerController 0)))

(event Input|KeyboardEvents|SpaceBar
  (params (Key :type Key%20Structure :default "None"))
  (:Pressed
    (Development|PrintString "PreseedSpace")))

(fn ConstructionScript
  (Variables|Default|SetSentenceReplace (Utilities|Struct|MakeSentenceReplace "Sam")))

(fn ReplaceText
  (params (NewParam :type Dialogue%20Structure))
  (Development|PrintString (Utilities|String|Replace (.DialgoueText (Utilities|Struct|BreakDialogueSentence (Utilities|Array|Get(acopy) (.Sentences (Utilities|Struct|BreakDialogue NewParam))))) "{playername}" "Sam")))

(fn InitializeNewDialogue
  (params (Dialogue :type Dialogue%20Structure))
  (|CallParentFunction Dialogue)
  ;[1 1 1] Open Dialogue
  (bind _asthird_person_character (Utilities|Casting|CastToThirdPersonCharacter (Game|Player|GetPlayerPawn 0)))
  (Default|StartDialogue (Variables|/Game/ThirdPersonCharacter_2020-08-28-21-01-43.ThirdPersonCharacter_C|GetPlayerHUD _asthird_person_character) (Variables|Default|GetCurrentDialogue))
  (Input|EnableInput (Game|GetPlayerController 0))
  (return))

(fn EndDialogue
  (bind _asthird_person_character (Utilities|Casting|CastToThirdPersonCharacter (Game|GetPlayerCharacter 0)))
  (Default|EndDialogue (Variables|/Game/ThirdPersonCharacter_2020-08-28-21-01-43.ThirdPersonCharacter_C|GetPlayerHUD _asthird_person_character)))