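; EnemyStart is an enemy actor Blueprint with a health module, a widget-component health bar and a capsule collider.
; On BeginPlay it passes the health module to the EnemyHealthbar widget so the widget can create its event bindings.
; When damage brings health to zero or below, it hides the bar and switches the capsule to the IgnoreOnlyPawn collision profile, leaving the actor in place.
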(event OnTakeDamage(HealthModule)
  (params (HealthPercentage :type Float%20%28single-precision%29))
  (if (<= HealthPercentage 0.0)
    (Rendering|SetVisibility (Variables|Default|GetHealthBar) false false)
    (Collision|SetCollisionProfileName (Variables|Default|GetCapsuleComponent) "IgnoreOnlyPawn" true :!class /Script/Engine.PrimitiveComponent)))

(event EventBeginPlay
  (bind _asenemy_healthbar (Utilities|Casting|CastToEnemyHealthbar (UserInterface|GetUserWidgetObject (Variables|Default|GetHealthBar))))
  (Default|CreateEvents _asenemy_healthbar (Variables|Default|GetHealthModule)))

(event Collision|EventActorBeginOverlap
  (params (OtherActor :type Actor%20Object%20Reference)))

(event EventTick
  (params (DeltaSeconds :type Float%20%28single-precision%29)))

(fn ConstructionScript)