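; Matchmaker NPC that offers itself as the current interactable to any overlapping actor with an InteractComponent.
; Its StartMatchMaking event is an empty stub, so interacting triggers no matchmaking here.
; An unwired Advanced Sessions chain searches for non-empty sessions and joins the first result, or creates one and opens the third-person example map as a listen server.
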(event OnComponentBeginOverlap(Sphere)
  (params (OverlappedComponent :type Primitive%20Component%20Object%20Reference) (OtherActor :type Actor%20Object%20Reference) (OtherComp :type Primitive%20Component%20Object%20Reference) (OtherBodyIndex :type Integer) (bFromSweep :type Boolean) (SweepResult :type Hit%20Result%20Structure%20%28by%20ref%29))
  (bind _returnvalue (Actor|GetComponentbyClass OtherActor "/Script/MobileGame.InteractComponent"))
  (Utilities|IsValid _returnvalue
    (:Is%20Valid
      (Class|InteractComponent|SetCurrentInteractable _returnvalue self))))

(event Custom|StartMatchMaking)

(fn ConstructionScript)